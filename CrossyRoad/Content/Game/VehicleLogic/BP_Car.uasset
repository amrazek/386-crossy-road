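; BP_Car is a car actor that drives itself along its local X axis with a randomly chosen body.
; The construction script adds one instance at the actor origin to a random InstancedStaticMeshComponent on the actor.
; The random index is bounded by the component count minus one, so the last component is never picked.
; Tick moves the root by Speed times delta seconds, with sweep enabled.
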(event EventBeginPlay)

(event Collision|EventActorBeginOverlap
  (params (OtherActor :type Actor%20Object%20Reference)))

(event EventTick
  (params (DeltaSeconds :type Float%20%28single-precision%29))
  (Transformation|AddLocalOffset (Variables|Default|GetDefaultSceneRoot) (Math|Vector|MakeVector (* DeltaSeconds (Variables|Default|Getspeed)) 0.0 0.0) true false))

(fn ConstructionScript
  (CallFunction|SpawnVehicle))

(fn SpawnVehicle
  (bind _returnvalue (Actor|GetComponentsByClass "/Script/Engine.InstancedStaticMeshComponent"))
  (Components|InstancedStaticMesh|AddInstance (Utilities|Array|Get(acopy) _returnvalue (Math|Random|RandomInteger (- (Utilities|Array|Length _returnvalue) 1))) (Math|Transform|MakeTransform "0, 0, 0" "0,0.000000, 0")))