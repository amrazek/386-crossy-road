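; Lane spawner that builds the level from water, road and grass lanes for the top-down game mode.
; BeginPlay gathers three spawners through BPI_TileSpawner and lays opening lanes with the water spawner, despite a comment saying grass.
; A loop comparing player lane plus chunk size to the last generated index adds random-type lane batches, advancing that game mode index.
; The player lane-change handler re-enters that loop, but its binding never runs.
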(event Custom|OnPlayerLaneIndexChanged
  (params (PlayerLaneIndex :type Integer))
  (bind _gamemode (Variables|Default|GetGameMode))
  ;[1 1 1] Spawns new lanes if player does not have at least 1 full chunk of lanes in front of them
  (while (< (+ (Variables|/Game/Game/GM_TopDown.GM_TopDown_C|GetChunkSize _gamemode) PlayerLaneIndex) (Variables|/Game/Game/GM_TopDown.GM_TopDown_C|GetLastGeneratedLaneIndex _gamemode))
    (CallFunction|SpawnNewLanes)))

(event EventBeginPlay
  (Utilities|FlowControl|Sequence
    (:then_0
      (Utilities|FlowControl|Sequence
        (:then_0
          (bind _asbpi_tile_spawner (Utilities|Casting|CastToBPI_TileSpawner (Variables|Default|GetWaterLaneSpawner))))
        (:then_1
          (bind _asbpi_tile_spawner_2 (Utilities|Casting|CastToBPI_TileSpawner (Variables|Default|GetRoadLaneSpawner))))
        (:then_2
          (bind _asbpi_tile_spawner_3 (Utilities|Casting|CastToBPI_TileSpawner (Variables|Default|GetGrassLaneSpawner))))))
    (:then_1
      (Variables|Default|SetTileSpawners (Utilities|Array|MakeArray _asbpi_tile_spawner _asbpi_tile_spawner_2 _asbpi_tile_spawner_3)))
    (:then_2
      (bind _asgm_top_down (Utilities|Casting|CastToGM_TopDown (Game|GetGameMode)))
      (bind _output_get (Variables|Default|SetGameMode _asgm_top_down)))
    (:then_3
      (CallFunction|SpawnInitialLanes (Variables|Default|GetTileSpawners)))
    (:then_5
      ;[1 1 1] Spawns new lanes if player does not have at least 1 full chunk of lanes in front of them
      (while (< (+ (Variables|/Game/Game/GM_TopDown.GM_TopDown_C|GetChunkSize (Variables|Default|GetGameMode)) (stale Custom|OnPlayerLaneIndexChanged PlayerLaneIndex)) (Variables|/Game/Game/GM_TopDown.GM_TopDown_C|GetLastGeneratedLaneIndex (Variables|Default|GetGameMode)))
        (CallFunction|SpawnNewLanes)))))

(event EventTick
  (params (DeltaSeconds :type Float%20%28single-precision%29)))

(fn ConstructionScript)

(fn SpawnNewLanes
  (bind _tilespawners (Variables|Default|GetTileSpawners))
  (bind _gamemode (Variables|Default|GetGameMode))
  (bind _numlanescreated (Default|SpawnLanes (Utilities|Array|Get(acopy) _tilespawners (Math|Random|RandomIntegerinRange 0 (- (Utilities|Array|Length _tilespawners) 1))) (Variables|/Game/Game/GM_TopDown.GM_TopDown_C|GetLastGeneratedLaneIndex _gamemode) 6 2 (Variables|/Game/Game/GM_TopDown.GM_TopDown_C|GetMaxTilesInLane _gamemode) (Variables|/Game/Game/GM_TopDown.GM_TopDown_C|GetPlayableTilesInLane _gamemode)))
  (Variables|/Game/Game/GM_TopDown.GM_TopDown_C|SetLastGeneratedLaneIndex _gamemode (+ (Variables|/Game/Game/GM_TopDown.GM_TopDown_C|GetLastGeneratedLaneIndex _gamemode) _numlanescreated)))

(fn SpawnInitialLanes
  (params (Spawners :type Array%20of%20BPI%20Tile%20Spawner%20Interfaces))
  (bind _gamemode (Variables|Default|GetGameMode))
  (bind _array_element (Utilities|Array|ForEachLoopwithBreak Spawners :!label _label)
    (:LoopBody
      (bind _asbp_water_lane_spawner (Utilities|Casting|CastToBP_WaterLaneSpawner _array_element))
      (if (Utilities|IsValid _asbp_water_lane_spawner)
        (LocalVariables|SetInitialSpawner _asbp_water_lane_spawner)
        (goto _label Break)))
    (:Completed
      (Utilities|FlowControl|Sequence
        (:then_0
          ;[1 1 1] Spawn a few grass lanes to start on
          (bind _numlanescreated (Default|SpawnLanes (LocalVariables|GetInitialSpawner) 0 (Variables|/Game/Game/GM_TopDown.GM_TopDown_C|GetChunkSize _gamemode) 3 (Variables|/Game/Game/GM_TopDown.GM_TopDown_C|GetMaxTilesInLane _gamemode) (Variables|/Game/Game/GM_TopDown.GM_TopDown_C|GetPlayableTilesInLane _gamemode)))
          (Variables|/Game/Game/GM_TopDown.GM_TopDown_C|SetLastGeneratedLaneIndex _gamemode (+ _numlanescreated (Variables|/Game/Game/GM_TopDown.GM_TopDown_C|GetLastGeneratedLaneIndex _gamemode))))))))