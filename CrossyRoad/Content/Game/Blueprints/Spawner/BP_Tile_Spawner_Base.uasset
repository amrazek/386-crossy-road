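; Base tile spawner that builds lanes of randomly chosen tile actors, caching the GM_TopDown game mode on BeginPlay.
; SpawnLanes spawns a random number of lanes through SpawnTileLane, which picks a random variation per tile and places it via GetTileTransform.
; Lane indices start at zero, ignoring StartLaneIndex, and PlayableWidth is unused.
; The returned count is a separate random roll, so it can differ from the lanes spawned.
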(event EventBeginPlay
  (bind _asgm_top_down (Utilities|Casting|CastToGM_TopDown (Game|GetGameMode)))
  (Variables|Default|SetGameMode _asgm_top_down))

(event EventTick
  (params (DeltaSeconds :type Float%20%28single-precision%29)))

(fn SpawnTileLane
  (params (LaneIndex :type Integer) (LaneWidth :type Integer) (TileVariations :type Array%20of%20Actor%20Class%20References))
  (for _index (range 0 (- LaneWidth 1))
    (bind _tiletransform (CallFunction|GetTileTransform (Variables|Default|GetGameMode) _index LaneIndex))
    (Game|SpawnActorfromClass (Utilities|Array|Get(acopy) TileVariations (Math|Random|RandomIntegerinRange 0 (- (Utilities|Array|Length TileVariations) 1))) _tiletransform "AlwaysSpawn" 0 0)))

(fn SpawnLanes
  (params (StartLaneIndex :type Integer) (MaxNewLanes :type Integer) (MinNewLanes :type Integer) (LaneWidth :type Integer) (PlayableWidth :type Integer))
  (bind _returnvalue (Math|Random|RandomIntegerinRange MinNewLanes MaxNewLanes))
  (for _index (range 0 (- _returnvalue 1))
    (CallFunction|SpawnTileLane (+ 0 _index) LaneWidth (Variables|Default|GetTileVariations)))
  (return _returnvalue))