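; Prototype player chicken that hops tile to tile across a lane-based map.
; Jump checks the target tile is passable, disables input, then launches the physics mesh with a ballistic velocity impulse timed by JumpTime.
; Hitting a "Ground"-tagged component while airborne snaps position and rotation to the grid, zeroes velocity, updates tile coordinates and re-enables input.
; Jumps to or from water lanes are unimplemented, only printing a TODO.
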(event OnComponentHit(ChickenMesh)
  (params (HitComponent :type Primitive%20Component%20Object%20Reference) (OtherActor :type Actor%20Object%20Reference) (OtherComp :type Primitive%20Component%20Object%20Reference) (NormalImpulse :type Vector :default "0, 0, 0") (Hit :type Hit%20Result%20Structure%20%28by%20ref%29))
  ;[1 1 1] Trigger On Landed
  (if (and (Components|ComponentHasTag OtherComp "Ground") (Variables|Default|GetIsAirborne))
    (Variables|Default|SetIsAirborne false)
    (CallFunction|OnLanded)))

(event Custom|OnLanded
  (bind _gamemode (Variables|Default|GetGameMode))
  (bind _chickenmesh (Variables|Default|GetChickenMesh))
  ;[1 1 1] On Landed Event
  (Utilities|FlowControl|Sequence
    (:then_0
      (bind _alignedworldposition (CallFunction|GetMapAlignedPosition (Transformation|GetActorLocation) _gamemode))
      (Transformation|SetActorLocation _alignedworldposition false true)
      (CallFunction|UpdateSelfLocationCoords))
    (:then_1
      (Class|PrimitiveComponent|SetAllPhysicsLinearVelocity _chickenmesh "0, 0, 0" false)
      (Class|PrimitiveComponent|SetAllPhysicsAngularVelocityinRadians _chickenmesh (Math|Vector|MakeVector 0.0 0.0 0.0) false))
    (:then_2
      (bind (_alignedrotation _compassdir) (CallFunction|GetMapAlignedRotation (Transformation|GetWorldRotation _chickenmesh) _gamemode))
      (Transformation|SetActorRotation _alignedrotation true)
      (Variables|Default|SetFacingDirection _compassdir))
    (:then_3
      (Input|EnableInput (Game|GetPlayerController 0) 0)
      (Development|PrintString "Landed on ground"))))

(event EventBeginPlay
  ;[1 1 1] Setup
  (Utilities|FlowControl|Sequence
    (:then_0
      (bind _asgm_top_down (Utilities|Casting|CastToGM_TopDown (Game|GetGameMode)))
      (Variables|Default|SetGameMode _asgm_top_down))
    (:then_1
      (Variables|Default|SetForwardImpulse (/ (.x (Variables|/Game/Blueprints/GM_TopDown.GM_TopDown_C|GetTileSize (Variables|Default|GetGameMode))) (Variables|Default|GetJumpTime))))
    (:then_2
      (CallFunction|UpdateSelfLocationCoords))))

(fn ConstructionScript)

(fn Jump
  (params (Direction :type E_Compass%20Enum :default "NewEnumerator0"))
  (if (not (Variables|Default|GetIsAirborne)) ; If already airborne, do nothing
    (bind _isjumpablelocation (CallFunction|CanJumpinDirection Direction))
    (if _isjumpablelocation
      (Utilities|FlowControl|Sequence
        (:then_0
          (Input|DisableInput (Game|GetPlayerController 0) 0))
        (:then_1
          (bind _canusecompassjump (CallFunction|IsSimpleGridMovement Direction))
          (if _canusecompassjump
            (bind _success (CallFunction|JumpUsingCompassDirection Direction))
            (else
              (Development|PrintString "TODO: non-compass jump"))))
        (:then_2
          (if _success
            (Variables|Default|SetIsAirborne true)
            (bind _outrotation (CallFunction|CompassDirectiontoRotation Direction))
            (Transformation|SetActorRotation _outrotation true))))
      (else
        (Development|PrintString "Can't jump in that direction")))))

(fn UpdateSelfLocationCoords
  (bind (_x _y) (CallFunction|GetTileCoordsfromMapSpacePosition (.location (Math|Transform|MakeRelativeTransform (Math|Transform|MakeTransform (.location (Transformation|GetActorTransform))) (Transformation|GetActorTransform (Variables|/Game/Blueprints/GM_TopDown.GM_TopDown_C|GetMapRoot (Variables|Default|GetGameMode))))) (Variables|/Game/Blueprints/GM_TopDown.GM_TopDown_C|GetTileSize (Variables|Default|GetGameMode))))
  (Utilities|FlowControl|Sequence
    (:then_0
      (Variables|Default|SetXLocation _x))
    (:then_1
      (Variables|Default|SetYLocation _y))))

(fn CanJumpinDirection
  (params (Direction :type E_Compass%20Enum :default "NewEnumerator0"))
  (bind (_relativexcoord _relativeycoord) (CallFunction|CompassDirectiontoRelativeTileCoord Direction))
  (bind (_lane _found) (Default|GetLanebyIndex (Variables|/Game/Blueprints/GM_TopDown.GM_TopDown_C|GetMapRoot (Variables|Default|GetGameMode)) (+ _relativeycoord (Variables|Default|GetYLocation))))
  (if _found
    (bind _ispassable (Default|GetPassable _lane (+ _relativexcoord (Variables|Default|GetXLocation)))))
  (return (and _found _ispassable)))

(fn CalculateTrajectoryImpulse
  (params (StartLocationWorld :type Vector) (TargetLocationWorld :type Vector))
  (bind _returnvalue (Math|Vector|Distance2D(Vector) (Math|Vector|MakeVector (.x StartLocationWorld) (.y StartLocationWorld) 0.0) (Math|Vector|MakeVector (.x TargetLocationWorld) (.y TargetLocationWorld) 0.0)))
  (bind _returnvalue_2 (Math|Vector|MakeVector (.x TargetLocationWorld) (.y TargetLocationWorld) 0.0))
  (bind _returnvalue_3 (Math|Vector|MakeVector (.x StartLocationWorld) (.y StartLocationWorld) 0.0))
  (bind _jumptime (Variables|Default|GetJumpTime))
  (bind _returnvalue_4 (- _returnvalue_2 _returnvalue_3))
  (bind _returnvalue_5 (/ _returnvalue _jumptime))
  (bind _returnvalue_6 (Math|Vector|Normalize _returnvalue_4))
  (bind _returnvalue_7 (* _returnvalue_6 _returnvalue_5))
  (return (Math|Vector|MakeVector (.x _returnvalue_7) (.y _returnvalue_7) (/ (- (- (.z TargetLocationWorld) (.z StartLocationWorld)) (* (* (* _jumptime _jumptime) (Variables|Default|GetGravity)) 0.5)) _jumptime))))

(fn JumpUsingCompassDirection
  (params (CompassDirection :type E_Compass%20Enum :default "NewEnumerator0"))
  (bind _gamemode (Variables|Default|GetGameMode))
  (bind _tilesize (Variables|/Game/Blueprints/GM_TopDown.GM_TopDown_C|GetTileSize _gamemode))
  (bind (_relativexcoord _relativeycoord) (CallFunction|CompassDirectiontoRelativeTileCoord CompassDirection))
  (bind (_lane _found) (Default|GetLanebyIndex (Variables|/Game/Blueprints/GM_TopDown.GM_TopDown_C|GetMapRoot (Variables|Default|GetGameMode)) (+ _relativeycoord (Variables|Default|GetYLocation))))
  (if _found
    (bind _impulseforcevelocity (CallFunction|CalculateTrajectoryImpulse (Math|Vector|MakeVector 0.0 0.0 (.z (Transformation|GetActorLocation))) (Math|Vector|MakeVector (* _relativeycoord (.x _tilesize)) (* _relativexcoord (.y _tilesize)) (.LaneZHeight (Utilities|Struct|BreakBPS_Spawner (Variables|/Game/Blueprints/Map/BP_LaneBase.BP_LaneBase_C|GetSpawnerInfo _lane))))))
    (Physics|AddImpulse (Variables|Default|GetChickenMesh) _impulseforcevelocity "None" true)
    (return true)
    (else
      (return false))))

(fn IsSimpleGridMovement
  (params (JumpDirection :type E_Compass%20Enum :default "NewEnumerator0"))
  (bind _ylocation (Variables|Default|GetYLocation))
  (bind _gamemode (Variables|Default|GetGameMode))
  (bind _maproot (Variables|/Game/Blueprints/GM_TopDown.GM_TopDown_C|GetMapRoot _gamemode))
  (bind _relativeycoord (CallFunction|CompassDirectiontoRelativeTileCoord JumpDirection))
  (bind (_lane _found) (Default|GetLanebyIndex _maproot (+ _ylocation _relativeycoord))) ; Target Lane
  (bind (_lane_2 _found_2) (Default|GetLanebyIndex _maproot _ylocation)) ; Own Lane
  (return (and _found_2 (== (.Spawner (Utilities|Struct|BreakBPS_Spawner (Variables|/Game/Blueprints/Map/BP_LaneBase.BP_LaneBase_C|GetSpawnerInfo _lane_2))) "/Game/Blueprints/Map/BP_WaterLane.BP_WaterLane_C")) (and (== (.Spawner (Utilities|Struct|BreakBPS_Spawner (Variables|/Game/Blueprints/Map/BP_LaneBase.BP_LaneBase_C|GetSpawnerInfo _lane))) "/Game/Blueprints/Map/BP_WaterLane.BP_WaterLane_C") _found) (and (not (and (== (.Spawner (Utilities|Struct|BreakBPS_Spawner (Variables|/Game/Blueprints/Map/BP_LaneBase.BP_LaneBase_C|GetSpawnerInfo _lane))) "/Game/Blueprints/Map/BP_WaterLane.BP_WaterLane_C") _found)) (not (and _found_2 (== (.Spawner (Utilities|Struct|BreakBPS_Spawner (Variables|/Game/Blueprints/Map/BP_LaneBase.BP_LaneBase_C|GetSpawnerInfo _lane_2))) "/Game/Blueprints/Map/BP_WaterLane.BP_WaterLane_C"))))))