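; BP_Eagle is an eagle actor that starts the GM_TopDown game-over sequence on BeginPlay and carries off a chicken.
; Tick moves it straight toward the Chicken reference until within a small radius, then destroys the chicken, reveals StaticMesh1 and plays a hit sound.
; With HasChicken set, it flies along negative X with a slight climb.
; The Attack function is empty, and a debug print remains.
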(event EventBeginPlay
  (bind _asgm_top_down (Utilities|Casting|CastToGM_TopDown (Game|GetGameMode)))
  (Variables|Default|SetGameMode _asgm_top_down)
  (Default|StartGameOverSequence (Variables|Default|GetGameMode)))

(event EventTick
  (params (DeltaSeconds :type Float%20%28single-precision%29))
  (bind _returnvalue (Transformation|GetActorLocation))
  (bind _chicken (Variables|Default|GetChicken))
  (bind _speed (Variables|Default|GetSpeed))
  (bind _chicken_2 (Variables|Default|GetChicken))
  (bind _returnvalue_2 (Transformation|GetActorLocation _chicken))
  (if (Variables|Default|GetHasChicken)
    (Transformation|AddActorWorldOffset (Math|Vector|MakeVector (* (* DeltaSeconds _speed) -1.0) 0.0 (* DeltaSeconds (* _speed 0.1))))
    (else
      (Utilities|IsValid _chicken
        (:Is%20Valid
          (if (<= (Math|Vector|Distance(Vector) _returnvalue_2 _returnvalue) 2e+01)
            (Development|PrintString "Hello")
            (Utilities|IsValid _chicken_2
              (:Is%20Valid
                (Actor|DestroyActor _chicken_2)
                (Rendering|SetVisibility (Variables|Default|GetStaticMesh1) true false)
                (Variables|Default|SetHasChicken true)
                (Audio|PlaySoundatLocation "/Game/Sounds/Eagle/eaglehit.eaglehit" (Transformation|GetActorLocation) "0, 0, 0" 1.0 1.0 0.0 0 0 0)))
            (else
              (Transformation|AddWorldOffset (Variables|Default|GetDefaultSceneRoot) (* (* (Math|Vector|Normalize (- _returnvalue_2 _returnvalue)) (Variables|Default|GetSpeed)) DeltaSeconds) false false))))))))

(fn ConstructionScript)

(fn Attack)