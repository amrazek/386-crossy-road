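; BP_GrassLane is a map lane actor that builds a row of grass tiles for the top-down game mode.
; On BeginPlay it loops over the game mode's lane tile count, adding flat grass instances inside the playable zone and darkened grass plus blocking trees outside it.
; Tiles and trees are instanced components placed by relative transform; the construction script assigns the darkened grass material.
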(event EventBeginPlay
  (bind _asgm_top_down (Utilities|Casting|CastToGM_TopDown (Game|GetGameMode)))
  (bind _output_get (Variables|Default|SetGameMode _asgm_top_down))
  (for _index (range 0 (- (Variables|/Game/Blueprints/GM_TopDown.GM_TopDown_C|GetMaxTilesInLane _output_get) 1))
    (bind _localtransform (CallFunction|GetTileTransformRelative _output_get _index))
    (bind _iswithinplayablezone (CallFunction|TileIsinPlayableZone _output_get _index))
    (if _iswithinplayablezone
      (Components|InstancedStaticMesh|AddInstance (Variables|Default|GetGrassFlat) _localtransform)
      (else
        (Components|InstancedStaticMesh|AddInstance (Variables|Default|GetGrassFlat_Dark) _localtransform)
        (Components|InstancedStaticMesh|AddInstance (Variables|Default|GetBlockingTree) _localtransform)))))

(event Collision|EventActorBeginOverlap
  (params (OtherActor :type Actor%20Object%20Reference)))

(event EventTick
  (params (DeltaSeconds :type Float%20%28single-precision%29)))

(fn ConstructionScript
  (Rendering|Material|SetMaterial (Variables|Default|GetGrassFlat_Dark) 0 "/Game/Tiles/M_grass_h3_darken.M_grass_h3_darken"))