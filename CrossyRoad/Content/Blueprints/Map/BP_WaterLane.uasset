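; Water lane for the chicken lane-crossing game, filled with either floating logs or lily pads, where touching the splash zone kills the chicken.
; BeginPlay checks the previous lane to prevent adjacent lily lanes, otherwise picking logs 66% of the time.
; It attaches a log spawner or randomly scatters lily pads, retrying until at least one exists.
; Every tile is marked passable, and whitewater emitters spawn at the playable area's border seams.
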(event OnComponentBeginOverlap(SplashZone)
  (params (OverlappedComponent :type Primitive%20Component%20Object%20Reference) (OtherActor :type Actor%20Object%20Reference) (OtherComp :type Primitive%20Component%20Object%20Reference) (OtherBodyIndex :type Integer) (bFromSweep :type Boolean) (SweepResult :type Hit%20Result%20Structure%20%28by%20ref%29))
  (Utilities|IsValid OtherActor
    (:Is%20Valid
      (bind _asbp_chicken (Utilities|Casting|CastToBP_Chicken OtherActor))
      (Default|Kill _asbp_chicken "NewEnumerator3"))))

(event EventBeginPlay
  (bind _ism_watertile (Variables|Default|GetISM_WaterTile))
  (bind _gamemode (Variables|Default|GetGameMode))
  (Utilities|FlowControl|Sequence
    (:then_1
      (Components|InstancedStaticMesh|ClearInstances (Variables|Default|GetISM_Lily_PreviewOnly))
      (Components|InstancedStaticMesh|ClearInstances (Variables|Default|GetISM_WaterTile)))
    (:then_2
      (Variables|Default|SetPassableGroundTile _ism_watertile))
    (:then_3
      (Variables|Default|SetImpassableGroundTile _ism_watertile))
    (:then_4
      (|CallParentFunction))
    (:then_5
      (bind (_lane _found) (Default|GetLanebyIndex (Variables|/Game/Blueprints/GM_TopDown.GM_TopDown_C|GetMapRoot _gamemode) (- (Variables|/Game/Blueprints/GM_TopDown.GM_TopDown_C|GetLanesSpawned _gamemode) 1)))
      (if _found
        (bind _asbp_water_lane (Utilities|Casting|CastToBP_WaterLane _lane)
          (:then
            (if (== (Variables|BP_WaterLane_C|GetLaneType _asbp_water_lane) (Utilities|Enum|LiteralenumE_WaterLaneType "NewEnumerator0"))
              ;[1 1 1] never allow two adjacent lily pad lanes
              (Variables|Default|SetSpawnsLogs true :!label _label)
              (CallFunction|SpawnLogs)
              (Variables|Default|SetLaneType "NewEnumerator1")
              (else
                (if (Math|Random|RandomBoolwithWeight 0.66) :!label _label_2
                  (goto _label)
                  (else
                    (Variables|Default|SetSpawnsLogs false)
                    (CallFunction|SpawnLilies)
                    (Variables|Default|SetLaneType "NewEnumerator0"))))))
          (:CastFailed
            (goto _label_2)))
        (else
          (goto _label_2))))))

(event EventOnTileSpawned
  (params (Index :type Integer) (IsPassable :type Boolean))
  ;[1 1 1] Spawn waterfalls (eventually)
  (Utilities|FlowControl|Sequence
    (:then_0
      (bind (_localposofseam _isborder) (CallFunction|IsBorderTile Index))
      (if _isborder
        (Effects|SpawnEmitterAttached "/Game/Blueprints/PS_WhiteWater.PS_WhiteWater" (Variables|Default|GetDefaultSceneRoot) "None" _localposofseam (Transformation|GetActorRotation))))
    (:then_1
      ;[1 1 1] Water lane always 'passable'
      (Utilities|Array|SetArrayElem (Variables|Default|GetLanePassability) Index true))))

(fn ConstructionScript
  (|CallParentFunction))

(fn IsBorderTile
  (params (Index :type Integer))
  (bind _gamemode (Variables|Default|GetGameMode))
  (bind _playabletilesinlane (Variables|/Game/Blueprints/GM_TopDown.GM_TopDown_C|GetPlayableTilesInLane _gamemode))
  (bind _maxtilesinlane (Variables|/Game/Blueprints/GM_TopDown.GM_TopDown_C|GetMaxTilesInLane _gamemode))
  (bind _tilesize (Variables|/Game/Blueprints/GM_TopDown.GM_TopDown_C|GetTileSize _gamemode))
  (bind _returnvalue (- _maxtilesinlane _playabletilesinlane))
  (bind _returnvalue_2 (/ (.y _tilesize) 2.0))
  (bind _returnvalue_3 (* Index (.y _tilesize)))
  (bind _returnvalue_4 (/ _returnvalue 2))
  (bind _returnvalue_5 (- _maxtilesinlane _returnvalue_4))
  (bind _returnvalue_6 (== Index _returnvalue_5))
  (if (or _returnvalue_6 (== Index _returnvalue_4))
    (if _returnvalue_6
      (return (+ (Math|Vector|MakeVector 0.0 _returnvalue_3 (.z _tilesize)) (Math|Vector|MakeVector 0.0 _returnvalue_2 0.0)) true)
      (else
        (return (- (Math|Vector|MakeVector 0.0 _returnvalue_3 (.z _tilesize)) (Math|Vector|MakeVector 0.0 _returnvalue_2 0.0)) true)))
    (else
      (return "0, 0, 0" false))))

(fn SpawnLilies
  (bind _gamemode (Variables|Default|GetGameMode))
  (bind _playabletilesinlane (Variables|/Game/Blueprints/GM_TopDown.GM_TopDown_C|GetPlayableTilesInLane _gamemode))
  (bind _maxtilesinlane (Variables|/Game/Blueprints/GM_TopDown.GM_TopDown_C|GetMaxTilesInLane _gamemode))
  (bind _returnvalue (/ _maxtilesinlane 2))
  (bind _returnvalue_2 (/ _playabletilesinlane 2))
  (bind _returnvalue_3 (- _returnvalue _returnvalue_2))
  (Utilities|FlowControl|Sequence
    (:then_0
      (for _index (range (- _returnvalue_3 1) (+ _returnvalue_3 _playabletilesinlane))
        (if (Math|Random|RandomBoolwithWeight 0.45)
          (bind _localtransform (CallFunction|GetTileTransformRelative (Variables|Default|GetGameMode) _index))
          (bind _returnvalue_4 (Game|SpawnActorfromClass "/Game/Blueprints/ObstacleSpawners/BP_LilyPad.BP_LilyPad_C" (Math|Transform|MakeTransform (.location _localtransform) (.rotation _localtransform) (.scale _localtransform)) "AlwaysSpawn" 0 0))
          (Transformation|AttachActorToActor _returnvalue_4 self "None" "KeepRelative" "KeepRelative" "KeepRelative" true)
          (Math|Integer|IncrementInt (LocalVariables|GetNumSpawned)))))
    (:then_1
      ;[1 1 1] Be sure there's at least one lily to use
      (if (== (LocalVariables|GetNumSpawned) 0)
        (CallFunction|SpawnLilies)))))

(fn SpawnLogs
  (Utilities|FlowControl|Sequence
    (:then_0
      (bind _worldtrans (CallFunction|GetObstacleSpawnerWorldTransform (Variables|Default|GetGameMode) self))
      (Variables|Default|SetSpawnerTransform _worldtrans))
    (:then_1
      (Variables|Default|SetSpawnsLogs true))
    (:then_2
      (bind _returnvalue (Game|SpawnActorfromClass "/Game/Blueprints/ObstacleSpawners/BP_LogSpawner.BP_LogSpawner_C" (Variables|Default|GetSpawnerTransform) "AlwaysSpawn" 0 0))
      (Transformation|AttachActorToActor _returnvalue self "None" "KeepWorld" "KeepWorld" "KeepWorld" true))))