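; BP_RoadLane is a road lane actor that supplies road ground tiles and hosts a vehicle spawner.
; On BeginPlay it runs the parent logic, assigns the passable and impassable road tiles, then calls SpawnLane.
; Once the lane finishes spawning, it creates a BP_VehicleSpawner at the computed obstacle spawner transform, passing in GameMode, and attaches it to itself.
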(event EventBeginPlay
  (Utilities|FlowControl|Sequence
    (:then_0
      (|CallParentFunction))
    (:then_1
      (Variables|Default|SetPassableGroundTile (Variables|Default|GetGroundPassable_Road))
      (Variables|Default|SetImpassableGroundTile (Variables|Default|GetGroundImpassable_Road)))
    (:then_2
      (CallFunction|SpawnLane))))

(event EventOnLaneFinishedSpawning
  (bind _self self)
  (bind _gamemode (Variables|Default|GetGameMode))
  (bind _worldtrans (CallFunction|GetObstacleSpawnerWorldTransform _gamemode _self))
  (bind _returnvalue (Game|SpawnActorfromClass "/Game/Blueprints/ObstacleSpawners/BP_VehicleSpawner.BP_VehicleSpawner_C" _worldtrans "DontSpawnIfColliding" 0 _gamemode 0))
  (Transformation|AttachActorToActor _returnvalue _self "None" "KeepWorld" "KeepWorld" "KeepWorld" true))

(fn ConstructionScript
  (|CallParentFunction))