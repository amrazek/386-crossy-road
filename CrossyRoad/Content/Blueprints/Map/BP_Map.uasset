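; Map actor that builds an endless lane-based playing area around the chicken.
; On BeginPlay it spawns starting grass lanes from LaneClasses, placing each along X using GM_TopDown's lane count and tile size.
; ExtendPlayingArea appends random lane types when the chicken nears the front edge and destroys lanes left behind.
; Spawned BP_LaneBase actors are attached, indexed in a map and told to build their own content.
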(event EventBeginPlay
  (bind _asgm_top_down (Utilities|Casting|CastToGM_TopDown (Game|GetGameMode)))
  (Variables|Default|SetGameMode _asgm_top_down)
  (CallFunction|SpawnInitialGrassLanes))

(fn ConstructionScript)

(fn SpawnMap
  (Utilities|FlowControl|Sequence
    (:then_0
      (CallFunction|SpawnInitialGrassLanes))
    (:then_1
      (for _index (range 0 10)
        (bind _selectedspawner (CallFunction|RandomlySelectLaneType))
        (CallFunction|SpawnLane _selectedspawner)))))

(fn SpawnInitialGrassLanes
  (Utilities|FlowControl|Sequence
    (:then_0
      (bind _array_element (Utilities|Array|ForEachLoopwithBreak (Variables|Default|GetLaneClasses) :!label _label)
        (:LoopBody
          (if (Utilities|Enum|Equal(Enum) (.Name (Utilities|Struct|BreakBPS_Spawner _array_element)) "Grass")
            (LocalVariables|SetGrassLaneSpawner _array_element)
            (goto _label Break)))))
    (:then_1
      (for _index (range 0 (- (Variables|Default|GetInitialGrassLanes) 1))
        (CallFunction|SpawnLane (LocalVariables|GetGrassLaneSpawner))))))

(fn SpawnLane
  (params (LaneSpawnerClass :type BPS%20Spawner%20Structure))
  (bind _gamemode (Variables|Default|GetGameMode))
  (bind _lanesspawned (Variables|/Game/Blueprints/GM_TopDown.GM_TopDown_C|GetLanesSpawned _gamemode))
  (Utilities|FlowControl|Sequence
    (:then_0
      (bind _returnvalue (Game|SpawnActorfromClass (.Spawner (Utilities|Struct|BreakBPS_Spawner LaneSpawnerClass)) (Math|Transform|MakeTransform (Math|Vector|MakeVector (* _lanesspawned (.x (Variables|/Game/Blueprints/GM_TopDown.GM_TopDown_C|GetTileSize _gamemode))) 0.0 0.0)) "AlwaysSpawn" 0 0))
      ;[1 1 1] Set Owner on SpawnActor doesn't seem to work
      (Transformation|AttachActorToActor _returnvalue self "None" "KeepRelative" "KeepRelative" "KeepRelative" true))
    (:then_1
      (bind _asbp_lane_base (Utilities|Casting|CastToBP_LaneBase _returnvalue)
        (:then
          (Utilities|Map|Add (Variables|Default|GetLanes) _lanesspawned _asbp_lane_base)
          (Variables|/Game/Blueprints/Map/BP_LaneBase.BP_LaneBase_C|SetSpawnerInfo _asbp_lane_base LaneSpawnerClass))
        (:CastFailed
          (Development|PrintString "ERROR: One of lane spawners is not a BP_LaneBase"))))
    (:then_2
      (Math|Integer|IncrementInt (Variables|/Game/Blueprints/GM_TopDown.GM_TopDown_C|GetLanesSpawned (Variables|Default|GetGameMode))))
    (:then_3
      (Default|SpawnLane _asbp_lane_base))))

(fn RandomlySelectLaneType
  (bind _laneclasses (Variables|Default|GetLaneClasses))
  (return (Utilities|Array|Get(acopy) _laneclasses (Math|Random|RandomIntegerinRange 0 (- (Utilities|Array|Length _laneclasses) 1)))))

(fn GetLanebyIndex
  (params (Index :type Integer))
  (bind _lanes (Variables|Default|GetLanes))
  (bind (_value _returnvalue) (Utilities|Map|Find _lanes Index))
  (return _value _returnvalue))

(fn ExtendPlayingArea
  (params (ChickenLocation :type Integer) (LanesSpawned :type Integer))
  (Utilities|FlowControl|Sequence
    (:then_0
      (if (< (- LanesSpawned ChickenLocation) 20)
        (for _index (range 0 9)
          (bind _selectedspawner (CallFunction|RandomlySelectLaneType))
          (CallFunction|SpawnLane _selectedspawner))))
    (:then_1
      (bind _keys (Utilities|Map|Keys (Variables|Default|GetLanes)))
      (for _array_element _keys
        (if (< _array_element (- ChickenLocation 7))
          (if (.ReturnValue (Utilities|Map|Find (Variables|Default|GetLanes) _array_element))
            (Utilities|Array|Add (LocalVariables|GetToDestroy) (.Value (Utilities|Map|Find (Variables|Default|GetLanes) _array_element)))))))
    (:then_2
      (bind _arrayelement (Utilities|Array|ReverseforEachLoop (LocalVariables|GetToDestroy))
        (:LoopBody
          (Utilities|IsValid _arrayelement
            (:Is%20Valid
              (Actor|DestroyActor _arrayelement))))
        (:Completed
          (Utilities|Array|Clear (LocalVariables|GetToDestroy)))))))