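; Blueprint function library of tile-grid helpers for a lane-based chicken crossing map.
; Converts between tile coordinates, map positions and compass directions using GameMode tile settings, with lanes along world X and tiles along world Y, and snaps positions and yaw to the grid.
; Also computes the chicken start point, playable-zone test and obstacle spawner transforms on a random lane end at lane height.
; RandomlyAddCoin occasionally picks a random passable tile for a coin.
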(fn CompassDirectiontoRelativeTileCoord
  (params (CompressDirection :type E_Compass%20Enum :default "NewEnumerator0"))
  (switch Utilities|FlowControl|Switch|SwitchonE_Compass CompressDirection
    (:NewEnumerator0
      (return 0 1))
    (:NewEnumerator1
      (return 1 0))
    (:NewEnumerator2
      (return 0 -1))
    (:NewEnumerator3
      (return -1 0))))

(fn CompassDirectiontoRotation
  (params (InDir :type E_Compass%20Enum :default "NewEnumerator0"))
  (switch Utilities|FlowControl|Switch|SwitchonE_Compass InDir
    (:NewEnumerator0
      (LocalVariables|SetYaw 0.0))
    (:NewEnumerator1
      (LocalVariables|SetYaw 9e+01))
    (:NewEnumerator2
      (LocalVariables|SetYaw 1.8e+02))
    (:NewEnumerator3
      (LocalVariables|SetYaw 2.7e+02)))
  (return (Math|Rotator|MakeRotator 0.0 0.0 (LocalVariables|GetYaw))))

(fn GetTileTransform
  (params (GameMode :type GM%20Top%20Down%20Object%20Reference) (TileIndexInLane :type Integer) (LaneIndex :type Integer))
  (bind _tilesize (Variables|/Game/Blueprints/GM_TopDown.GM_TopDown_C|GetTileSize GameMode))
  (return (Math|Transform|MakeTransform (Math|Vector|MakeVector (* LaneIndex (.x _tilesize)) (* TileIndexInLane (.y _tilesize)) 0.0))))

(fn GetObstacleSpawnerWorldTransform
  (params (GameMode :type GM%20Top%20Down%20Object%20Reference) (Owner :type Actor%20Object%20Reference))
  (bind _returnvalue (Transformation|GetActorTransform Owner))
  (bind ___worldcontext (LocalVariables|Get__WorldContext))
  (Utilities|FlowControl|Sequence
    (:then_0
      (bind _array_element (Utilities|Array|ForEachLoopwithBreak (Variables|/Game/Blueprints/Map/BP_Map.BP_Map_C|GetLaneClasses (Variables|/Game/Blueprints/GM_TopDown.GM_TopDown_C|GetMapRoot GameMode)) :!label _label)
        (:LoopBody
          (if (== (Utilities|GetClass Owner) (.Spawner (Utilities|Struct|BreakBPS_Spawner _array_element)))
            (LocalVariables|SetZOffset (.LaneZHeight (Utilities|Struct|BreakBPS_Spawner _array_element)))
            (goto _label Break)))))
    (:then_1
      (switch int (Math|Random|RandomIntegerinRange 0 1)
        (:Default
          (bind _localtransform (CallFunction|GetTileTransformRelative GameMode 0 ___worldcontext :!label _label_2))
          (LocalVariables|SetSpawnTransform (Math|Transform|MakeTransform (+ (.location _returnvalue) (.location _localtransform)) (.rotation _returnvalue) (.scale _returnvalue)))
          (LocalVariables|SetIsLeftSide true))
        (:0
          (goto _label_2))
        (:1
          (bind _localtransform_2 (CallFunction|GetTileTransformRelative GameMode (- (Variables|/Game/Blueprints/GM_TopDown.GM_TopDown_C|GetMaxTilesInLane GameMode) 1) ___worldcontext))
          (LocalVariables|SetSpawnTransform (Math|Transform|MakeTransform (+ (.location _localtransform_2) (.location _returnvalue)) (.rotation _returnvalue) (.scale _returnvalue)))
          (LocalVariables|SetIsLeftSide false)))
      (Utilities|FlowControl|Sequence
        (:then_0
          (LocalVariables|SetSpawnTransform (Math|Transform|MakeTransform (Math|Vector|MakeVector (.x (.location (LocalVariables|GetSpawnTransform))) (.y (.location (LocalVariables|GetSpawnTransform))) (+ (.z (.location (LocalVariables|GetSpawnTransform))) (LocalVariables|GetZOffset))) (.rotation (LocalVariables|GetSpawnTransform)) (.scale (LocalVariables|GetSpawnTransform)))))
        (:then_1
          (if (LocalVariables|GetIsLeftSide)
            (LocalVariables|SetYawAngle 9e+01)
            (else
              (LocalVariables|SetYawAngle -9e+01)))
          (return (Math|Transform|MakeTransform (.Location (Math|Transform|BreakTransform (LocalVariables|GetSpawnTransform))) (Math|Rotator|CombineRotators (.Rotation (Math|Transform|BreakTransform (LocalVariables|GetSpawnTransform))) (Math|Rotator|MakeRotator 0.0 0.0 (LocalVariables|GetYawAngle))) (.Scale (Math|Transform|BreakTransform (LocalVariables|GetSpawnTransform)))) (LocalVariables|GetIsLeftSide)) ; IsLeft = spawner on left side of map
        )))))

(fn GetTileTransformRelative
  (params (GameMode :type GM%20Top%20Down%20Object%20Reference) (TileIndex :type Integer))
  (return (Math|Transform|MakeTransform (Math|Vector|MakeVector 0.0 (* TileIndex (.y (Variables|/Game/Blueprints/GM_TopDown.GM_TopDown_C|GetTileSize GameMode))) 0.0))))

(fn GetLaneWorldPosition
  (params (GameMode :type GM%20Top%20Down%20Object%20Reference) (LaneIndex :type Integer))
  (bind _tilesize (Variables|/Game/Blueprints/GM_TopDown.GM_TopDown_C|GetTileSize GameMode))
  (return (Math|Transform|MakeTransform (Math|Vector|MakeVector (* LaneIndex (.x _tilesize)) (* (/ (Variables|/Game/Blueprints/GM_TopDown.GM_TopDown_C|GetMaxTilesInLane GameMode) -2) (.y _tilesize)) 0.0))))

(fn GetTileCoordsfromMapSpacePosition
  (params (WorldPos :type Vector) (TileSize :type Vector))
  (return (.ReturnValue (Math|Float|Division(WholeandRemainder) (+ (.y WorldPos) (* (.x TileSize) 0.5)) (.y TileSize))) (.ReturnValue (Math|Float|Division(WholeandRemainder) (+ (* (.y TileSize) 0.5) (.x WorldPos)) (.x TileSize)))))

(fn GetMapSpacePositionfromTileCoords
  (params (X :type Integer) (Y :type Integer) (TileSize :type Vector))
  (return (Math|Vector|MakeVector (* Y (.x TileSize)) (* X (.y TileSize)) 0.0)))

(fn GetChickenStartPosition
  (params (Map :type BP%20Map%20Object%20Reference) (GameMode :type GM%20Top%20Down%20Object%20Reference))
  (bind _mapspacepos (CallFunction|GetMapSpacePositionfromTileCoords (/ (Variables|/Game/Blueprints/GM_TopDown.GM_TopDown_C|GetMaxTilesInLane GameMode) 2) 0 (Variables|/Game/Blueprints/GM_TopDown.GM_TopDown_C|GetTileSize GameMode) (LocalVariables|Get__WorldContext)))
  (return (+ (+ (Transformation|GetWorldLocation (Variables|/Game/Blueprints/Map/BP_Map.BP_Map_C|GetDefaultSceneRoot Map)) _mapspacepos) "0, 0,500.000000")))

(fn GetMapAlignedPosition
  (params (WorldPosition :type Vector) (GameMode :type GM%20Top%20Down%20Object%20Reference))
  (bind _maproot (Variables|/Game/Blueprints/GM_TopDown.GM_TopDown_C|GetMapRoot GameMode))
  (bind _tilesize (Variables|/Game/Blueprints/GM_TopDown.GM_TopDown_C|GetTileSize GameMode))
  (bind _returnvalue (Transformation|GetActorLocation _maproot))
  (bind _output_get (LocalVariables|SetOriginalWorldPos WorldPosition))
  (bind (_x _y) (CallFunction|GetTileCoordsfromMapSpacePosition (- WorldPosition _returnvalue) (Variables|/Game/Blueprints/GM_TopDown.GM_TopDown_C|GetTileSize GameMode) (LocalVariables|Get__WorldContext)))
  (return (+ (Math|Vector|MakeVector (* _y (.x _tilesize)) (* _x (.y _tilesize)) (.z _output_get)) _returnvalue)))

(fn GetMapAlignedRotation
  (params (Rotation :type Rotator) (GameMode :type GM%20Top%20Down%20Object%20Reference))
  (bind _returnvalue (+ (.yaw Rotation) 45.0))
  (bind _returnvalue_2 (/ _returnvalue 9e+01))
  (bind _returnvalue_3 (Math|Float|Floor _returnvalue_2))
  (switch int _returnvalue_3
    (:Default
      (LocalVariables|SetDir "NewEnumerator0" :!label _label))
    (:0
      (goto _label))
    (:1
      (LocalVariables|SetDir "NewEnumerator1"))
    (:2
      (LocalVariables|SetDir "NewEnumerator2"))
    (:3
      (LocalVariables|SetDir "NewEnumerator3")))
  (return (Math|Rotator|MakeRotator 0.0 0.0 (* _returnvalue_3 9e+01)) (LocalVariables|GetDir)))

(fn TileIsinPlayableZone
  (params (GameMode :type GM%20Top%20Down%20Object%20Reference) (TileIndex :type Integer))
  (bind _playabletilesinlane (Variables|/Game/Blueprints/GM_TopDown.GM_TopDown_C|GetPlayableTilesInLane GameMode))
  (bind _maxtilesinlane (Variables|/Game/Blueprints/GM_TopDown.GM_TopDown_C|GetMaxTilesInLane GameMode))
  (bind _returnvalue (- _maxtilesinlane _playabletilesinlane))
  (bind _returnvalue_2 (/ _returnvalue 2))
  (return (Math|Integer|InRange(Integer) TileIndex _returnvalue_2 (- _maxtilesinlane _returnvalue_2))))

(fn WorldPositiontoCompassDirection
  (params (ChickenLocation :type Vector) (TargetLocation :type Vector))
  (bind _returnvalue (Math|Vector|ProjectVectorontoPlane TargetLocation "0, 0,1.000000"))
  (bind _returnvalue_2 (Math|Vector|ProjectVectorontoPlane ChickenLocation "0, 0,1.000000"))
  (bind _returnvalue_3 (- (.y _returnvalue) (.y _returnvalue_2)))
  (bind _returnvalue_4 (- (.x _returnvalue) (.x _returnvalue_2)))
  (if (> (Math|Float|Absolute(Float) _returnvalue_4) (Math|Float|Absolute(Float) _returnvalue_3))
    (if (>= _returnvalue_4 0.0)
      (LocalVariables|SetCompassDir "NewEnumerator0")
      (else
        (LocalVariables|SetCompassDir "NewEnumerator2")))
    (elif (>= _returnvalue_3 0.0)
      (LocalVariables|SetCompassDir "NewEnumerator1")
      (else
        (LocalVariables|SetCompassDir "NewEnumerator3"))))
  (return (LocalVariables|GetCompassDir)))

(fn RandomlyAddCoin
  (params (Lane :type BP%20Lane%20Base%20Object%20Reference) (GameMode :type GM%20Top%20Down%20Object%20Reference) (LaneHeight :type Float%20%28single-precision%29))
  (if (Math|Random|RandomBoolwithWeight 0.1)
    (while (not (LocalVariables|GetDepositedCoin))
      (bind _output_get (LocalVariables|SetCoinTileIndex (Math|Random|RandomIntegerinRange 0 (- (Variables|/Game/Blueprints/GM_TopDown.GM_TopDown_C|GetMaxTilesInLane GameMode) 1))))
      (bind _ispassable (Default|GetPassable Lane _output_get))
      (if _ispassable
        (LocalVariables|SetDepositedCoin true)
        (bind _localtransform (CallFunction|GetTileTransformRelative GameMode _output_get))
        (return (Math|Transform|MakeTransform (+ (.Location (Math|Transform|BreakTransform _localtransform)) (Math|Vector|MakeVector 0.0 0.0 LaneHeight)) (Math|Rotator|CombineRotators (.Rotation (Math|Transform|BreakTransform _localtransform)) "0,90.000000, 0") (.Scale (Math|Transform|BreakTransform _localtransform))) true)))
    (else
      (return (Math|Transform|MakeTransform "0, 0, 0") false))))