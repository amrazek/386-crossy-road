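; Player chicken for a tile-and-lane hopping game, moved by timed physics impulses, with a Kill routine that spawns feathers and ends the game.
; Jump checks lane passability, then targets a tile or, on water lanes, box-traces for BPI_Landable points predicted from their velocity.
; A ballistic impulse launches it with input disabled; hitting Ground zeroes velocity, aligns rotation, snaps grid jumps to tiles and restores input.
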(event OnComponentHit(ChickenMesh)
  (params (HitComponent :type Primitive%20Component%20Object%20Reference) (OtherActor :type Actor%20Object%20Reference) (OtherComp :type Primitive%20Component%20Object%20Reference) (NormalImpulse :type Vector :default "0, 0, 0") (Hit :type Hit%20Result%20Structure%20%28by%20ref%29))
  ;[1 1 1] Trigger On Landed
  (if (and (Components|ComponentHasTag OtherComp "Ground") (Variables|Default|GetIsAirborne))
    (Variables|Default|SetIsAirborne false)
    (CallFunction|OnLanded)))

(event Custom|OnLanded
  (bind _gamemode (Variables|Default|GetGameMode))
  (bind _chickenmesh (Variables|Default|GetChickenMesh))
  ;[1 1 1] On Landed Event
  (Utilities|FlowControl|Sequence
    (:then_0
      (if (Variables|Default|GetIsOnGrid)
        (bind _alignedworldposition (CallFunction|GetMapAlignedPosition (Transformation|GetActorLocation) _gamemode))
        (Transformation|SetActorLocation _alignedworldposition false true))
      (CallFunction|UpdateSelfLocationCoords))
    (:then_1
      (Class|PrimitiveComponent|SetAllPhysicsLinearVelocity _chickenmesh "0, 0, 0" false)
      (Class|PrimitiveComponent|SetAllPhysicsAngularVelocityinRadians _chickenmesh (Math|Vector|MakeVector 0.0 0.0 0.0) false))
    (:then_2
      (bind (_alignedrotation _compassdir) (CallFunction|GetMapAlignedRotation (Transformation|GetWorldRotation _chickenmesh) _gamemode))
      (Transformation|SetActorRotation _alignedrotation true)
      (Variables|Default|SetFacingDirection _compassdir))
    (:then_3
      (Input|EnableInput (Game|GetPlayerController 0) 0))
    (:then_4
      (Default|CallLanded))))

(event EventBeginPlay
  ;[1 1 1] Setup
  (Utilities|FlowControl|Sequence
    (:then_0
      (bind _asgm_top_down (Utilities|Casting|CastToGM_TopDown (Game|GetGameMode)))
      (Variables|Default|SetGameMode _asgm_top_down))
    (:then_1
      (Variables|Default|SetForwardImpulse (/ (.x (Variables|/Game/Blueprints/GM_TopDown.GM_TopDown_C|GetTileSize (Variables|Default|GetGameMode))) (Variables|Default|GetJumpTime))))
    (:then_2
      (CallFunction|UpdateSelfLocationCoords))))

(fn ConstructionScript)

(fn Jump
  (params (Direction :type E_Compass%20Enum :default "NewEnumerator0"))
  (if (not (Variables|Default|GetIsAirborne))
    (Utilities|FlowControl|Sequence
      (:then_0
        (bind (_targetlocation _isvalidjump _isongrid) (CallFunction|SweepforLandingLocation Direction))
        (if _isvalidjump
          (Utilities|FlowControl|Sequence
            (:then_0
              (Variables|Default|SetIsOnGrid _isongrid))
            (:then_1
              (Variables|Default|SetIsAirborne true))
            (:then_2
              (Input|DisableInput (Game|GetPlayerController 0) 0))
            (:then_3
              (bind _outrotation (CallFunction|CompassDirectiontoRotation Direction))
              (Transformation|SetActorRotation _outrotation true))
            (:then_4
              (bind _impulseforcevelocity (CallFunction|CalculateTrajectoryImpulse (Transformation|GetWorldLocation (Variables|Default|GetChickenMesh)) _targetlocation))
              (Physics|AddImpulse (Variables|Default|GetChickenMesh) _impulseforcevelocity "None" true)
              (Default|CallJumped))))))))

(fn UpdateSelfLocationCoords
  (bind (_x _y) (CallFunction|GetTileCoordsfromMapSpacePosition (.location (Math|Transform|MakeRelativeTransform (Math|Transform|MakeTransform (.location (Transformation|GetActorTransform))) (Transformation|GetActorTransform (Variables|/Game/Blueprints/GM_TopDown.GM_TopDown_C|GetMapRoot (Variables|Default|GetGameMode))))) (Variables|/Game/Blueprints/GM_TopDown.GM_TopDown_C|GetTileSize (Variables|Default|GetGameMode))))
  (Utilities|FlowControl|Sequence
    (:then_0
      (Variables|Default|SetXLocation _x))
    (:then_1
      (Variables|Default|SetYLocation _y))
    (:then_2
      (Development|PrintString (Utilities|String|Append (Utilities|String|MakeLiteralString "Coords are now  ") (Utilities|String|Append (Utilities|String|Append (Utilities|String|ToString(Integer) _x) ",") (Utilities|String|ToString(Integer) _y)))))))

(fn CalculateTrajectoryImpulse
  (params (StartLocationWorld :type Vector) (TargetLocationWorld :type Vector))
  (bind _returnvalue (Math|Vector|Distance2D(Vector) (Math|Vector|MakeVector (.x StartLocationWorld) (.y StartLocationWorld) 0.0) (Math|Vector|MakeVector (.x TargetLocationWorld) (.y TargetLocationWorld) 0.0)))
  (bind _returnvalue_2 (Math|Vector|MakeVector (.x TargetLocationWorld) (.y TargetLocationWorld) 0.0))
  (bind _returnvalue_3 (Math|Vector|MakeVector (.x StartLocationWorld) (.y StartLocationWorld) 0.0))
  (bind _jumptime (Variables|Default|GetJumpTime))
  (bind _returnvalue_4 (- _returnvalue_2 _returnvalue_3))
  (bind _returnvalue_5 (/ _returnvalue _jumptime))
  (bind _returnvalue_6 (Math|Vector|Normalize _returnvalue_4))
  (bind _returnvalue_7 (* _returnvalue_6 _returnvalue_5))
  (return (Math|Vector|MakeVector (.x _returnvalue_7) (.y _returnvalue_7) (/ (- (- (.z TargetLocationWorld) (.z StartLocationWorld)) (* (* (* _jumptime _jumptime) (Variables|Default|GetGravity)) 0.5)) _jumptime))))

(fn Kill
  (params (Death%20Type :type E_DeathAnimations%20Enum :default "NewEnumerator0"))
  (bind _returnvalue (Transformation|GetActorTransform))
  (if (not (Variables|Default|GetDead))
    (Utilities|FlowControl|Sequence
      (:then_0
        (Variables|Default|SetDead true)
        (Rendering|SetVisibility (Variables|Default|GetChickenMesh) false true))
      (:then_1
        (switch Utilities|FlowControl|Switch|SwitchonE_DeathAnimations Death%20Type
          (:NewEnumerator0
            _)
          (:NewEnumerator1
            _)
          (:NewEnumerator2
            _)
          (:NewEnumerator3
            _))
        (Effects|SpawnEmitteratLocation "/Game/Blueprints/PS_Feathers.PS_Feathers" (.location _returnvalue) (.rotation _returnvalue) (.scale _returnvalue)))
      (:then_2
        (Default|SetGameOver (Variables|Default|GetGameMode)))
      (:then_3
        (Default|CallKilled)
        (Actor|DestroyActor)))))

(fn SweepforLandingLocation
  (params (Direction :type E_Compass%20Enum :default "NewEnumerator0"))
  (bind _returnvalue (Transformation|GetActorLocation))
  (bind _gamemode (Variables|Default|GetGameMode))
  (bind _gamemode_2 (Variables|Default|GetGameMode))
  (bind _chickenmesh (Variables|Default|GetChickenMesh))
  (bind _returnvalue_2 (Transformation|GetWorldLocation _chickenmesh))
  (bind _tilesize (Variables|/Game/Blueprints/GM_TopDown.GM_TopDown_C|GetTileSize _gamemode_2))
  (bind _tilesize_2 (Variables|/Game/Blueprints/GM_TopDown.GM_TopDown_C|GetTileSize _gamemode))
  (CallFunction|UpdateSelfLocationCoords)
  (bind (_relativexcoord _relativeycoord) (CallFunction|CompassDirectiontoRelativeTileCoord Direction))
  (bind _outrotation (CallFunction|CompassDirectiontoRotation Direction))
  (LocalVariables|SetChickenForwardTileUnaligned (+ (Math|Vector|MakeVector (.x _returnvalue) (.y _returnvalue) 0.0) (Math|Vector|RotateVector (Math|Vector|MakeVector (.x _tilesize) 0.0 0.0) _outrotation)))
  ;[1 1 1] Jump is allowed?
  (bind (_lane _found) (Default|GetLanebyIndex (Variables|/Game/Blueprints/GM_TopDown.GM_TopDown_C|GetMapRoot (Variables|Default|GetGameMode)) (+ _relativeycoord (Variables|Default|GetYLocation))))
  (if _found
    (if (Utilities|Array|Get(acopy) (Variables|/Game/Blueprints/Map/BP_LaneBase.BP_LaneBase_C|GetLanePassability _lane) (+ _relativexcoord (Variables|Default|GetXLocation)))
      ;[1 1 1] Grid jump or physics jump?
      (if (== (.Spawner (Utilities|Struct|BreakBPS_Spawner (Variables|/Game/Blueprints/Map/BP_LaneBase.BP_LaneBase_C|GetSpawnerInfo _lane))) "/Game/Blueprints/Map/BP_WaterLane.BP_WaterLane_C")
        (bind (_outhits _returnvalue_3) (Class|KismetSystemLibrary|BoxTraceMulti (LocalVariables|GetChickenForwardTileUnaligned) (+ (* (Math|Vector|GetForwardVector _outrotation) 0.01) (LocalVariables|GetChickenForwardTileUnaligned)) (Math|Vector|MakeVector (* (.y _tilesize) 0.33) (* (* (.x _tilesize) 0.5) 1.5) 32.0) "0, 0, 0" "TraceTypeQuery4" true 0 "Persistent" true))
        ;[1 1 1] Find closest thing to land on, if there are multiple possibilities. We consider velocity here
        (if _returnvalue_3
          (for _array_element _outhits
            (bind (_haslandingpoints _nearestpredictedlandingpoint) (CallFunction|GetNearestLandingMarker (.HitActor (Collision|BreakHitResult _array_element))))
            (if _haslandingpoints
              (LocalVariables|SetLandingActorPredictedLocation _nearestpredictedlandingpoint)
              (LocalVariables|SetLandingActorRef (.HitActor (Collision|BreakHitResult _array_element)))))
          (Utilities|IsValid (LocalVariables|GetLandingActorRef)
            (:Is%20Valid
              (return (LocalVariables|GetLandingActorPredictedLocation) true false))
            (:Is%20Not%20Valid
              _)))
        ;[1 1 1] Aim for a grid coordinate, even though we know nothing's there
        (bind _alignedworldposition (CallFunction|GetMapAlignedPosition (LocalVariables|GetChickenForwardTileUnaligned) (Variables|Default|GetGameMode)))
        (return (Math|Vector|MakeVector (.x _alignedworldposition) (.y _alignedworldposition) 1e+01) false false)
        (else
          ;[1 1 1] Target is a tile coordinate
          (return (+ (Math|Vector|MakeVector (.x _returnvalue_2) (.y _returnvalue_2) 0.0) (Math|Vector|MakeVector (* _relativeycoord (.x _tilesize_2)) (* _relativexcoord (.y _tilesize_2)) (.LaneZHeight (Utilities|Struct|BreakBPS_Spawner (Variables|/Game/Blueprints/Map/BP_LaneBase.BP_LaneBase_C|GetSpawnerInfo _lane))))) true true)))
      (else
        _)))
  (return "0, 0, 0" false (Variables|Default|GetIsOnGrid)))

(fn GetNearestLandingMarker
  (params (Target :type Actor%20Object%20Reference))
  (bind _returnvalue (Transformation|GetActorLocation))
  (if (Utilities|DoesObjectImplementInterface Target "/Game/Blueprints/ObstacleSpawners/BPI_Landable.BPI_Landable_C")
    (bind _velocityvector (Class|BPILandable|GetLandingPointVelocity(Message) Target))
    (bind _landingpoints (Class|BPILandable|GetLandingPoints(Message) Target))
    (if (> (Utilities|Array|Length _landingpoints) 0)
      (LocalVariables|SetNearest "100000.000000,1000000.000000,100000.000000")
      (for _array_element _landingpoints
        (if (< (Class|KismetMathLibrary|VectorDistance2DSquared (+ (Transformation|GetWorldLocation _array_element) (* _velocityvector (Variables|Default|GetJumpTime))) _returnvalue) (Class|KismetMathLibrary|VectorDistance2DSquared _returnvalue (LocalVariables|GetNearest)))
          (bind _output_get (LocalVariables|SetNearest (+ (Transformation|GetWorldLocation _array_element) (* _velocityvector (Variables|Default|GetJumpTime)))))))
      (return true _output_get)
      (else
        _)))
  (return false "0, 0, 0"))