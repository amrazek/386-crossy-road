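; BP_Chicken_Pawn is a physics-driven chicken pawn with a skeletal mesh and an unfinished jump.
; BeginPlay enables collision, and hits on a component tagged Ground zero the mesh's linear velocity and print a debug message.
; Jump only disables input for player controller 0; its Direction input is unused and a fixed forward-and-up impulse node sits disconnected, so it never launches the chicken.
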(event OnComponentHit(SkeletalMesh)
  (params (HitComponent :type Primitive%20Component%20Object%20Reference) (OtherActor :type Actor%20Object%20Reference) (OtherComp :type Primitive%20Component%20Object%20Reference) (NormalImpulse :type Vector :default "0, 0, 0") (Hit :type Hit%20Result%20Structure%20%28by%20ref%29)))

(event EventBeginPlay
  (Collision|SetActorEnableCollision true))

(event Collision|EventActorBeginOverlap
  (params (OtherActor :type Actor%20Object%20Reference)))

(event EventTick
  (params (DeltaSeconds :type Float%20%28single-precision%29)))

(event Collision|EventHit
  (params (MyComp :type Primitive%20Component%20Object%20Reference) (Other :type Actor%20Object%20Reference) (OtherComp :type Primitive%20Component%20Object%20Reference) (bSelfMoved :type Boolean) (HitLocation :type Vector :default "0, 0, 0") (HitNormal :type Vector :default "0, 0, 0") (NormalImpulse :type Vector :default "0, 0, 0") (Hit :type Hit%20Result%20Structure%20%28by%20ref%29))
  (if (Components|ComponentHasTag (.HitComponent (Collision|BreakHitResult Hit)) "Ground")
    (Physics|SetPhysicsLinearVelocity (Variables|Default|GetSkeletalMesh) "0, 0, 0" false "None")
    (Development|PrintString "Grounded")))

(fn ConstructionScript)

(fn Jump
  (params (Direction :type E_Compass%20Enum :default "NewEnumerator0"))
  (Input|DisableInput (Game|GetPlayerController 0)))