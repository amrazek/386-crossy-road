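; Obstacle spawner that sends a stream of cars along a tiled lane at one random speed picked at BeginPlay.
; A self-rescheduling random-delay timer calls Spawn, which adds an instance at the local origin of a random vehicle InstancedStaticMeshComponent and includes debug spacing prints.
; Tick advances instances, removes those beyond the lane length from GameMode tile settings, and aims to dirty render state only on each component's last instance.
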(event Custom|SpawnVehicle_Event
  (CallFunction|Spawn (Variables|Default|Getelapsed))
  (Variables|Default|Setelapsed 0.0)
  (Utilities|Time|SetTimerbyEvent (delegate Custom|SpawnVehicle_Event) (Math|Random|RandomFloatinRange (Variables|Default|GetMinSpawnDelay) (Variables|Default|GetMaxSpawnDelay))) ; no loop intended
)

(event EventBeginPlay
  (bind _gamemode (Variables|Default|GetGameMode))
  (Utilities|FlowControl|Sequence
    (:then_0
      (Variables|Default|SetVehicle_ISMs (Actor|GetComponentsByClass "/Script/Engine.InstancedStaticMeshComponent"))
      (Variables|Default|SetSpeed (Math|Random|RandomFloatinRange (Variables|Default|GetMinSpeed) (Variables|Default|GetMaxSpeed))))
    (:then_1
      ;[1 1 1] Set vehicle bounds
      (Variables|Default|SetTravelDistance (* (Math|Conversions|ToFloat(Integer) (Variables|/Game/Blueprints/GM_TopDown.GM_TopDown_C|GetMaxTilesInLane _gamemode)) (.y (Variables|/Game/Blueprints/GM_TopDown.GM_TopDown_C|GetTileSize _gamemode)))))
    (:then_3
      (Utilities|Time|SetTimerbyEvent (delegate Custom|SpawnVehicle_Event) (Math|Random|RandomFloatinRange (Variables|Default|GetMinSpawnDelay) (Variables|Default|GetMaxSpawnDelay))) ; no loop intended
    )))

(event Collision|EventActorBeginOverlap
  (params (OtherActor :type Actor%20Object%20Reference)))

(event EventTick
  (params (DeltaSeconds :type Float%20%28single-precision%29))
  (Variables|Default|Setelapsed (+ DeltaSeconds (Variables|Default|Getelapsed)))
  (CallFunction|UpdateVehiclePositions DeltaSeconds))

(fn ConstructionScript)

(fn UpdateVehiclePositions
  (params (Delta%20Seconds :type Float%20%28single-precision%29))
  (for _array_element (Variables|Default|GetVehicle_ISMs)
    (LocalVariables|SetLastInstanceIndex (- (Components|InstancedStaticMesh|GetInstanceCount _array_element) 1))
    (LocalVariables|SetDestructionCounter 0)
    (bind _index (Utilities|FlowControl|ForLoopwithBreak 0 (- (Components|InstancedStaticMesh|GetInstanceCount _array_element) 1))
      (:LoopBody
        (Utilities|FlowControl|Sequence
          (:then_0
            (if (.ReturnValue (Components|InstancedStaticMesh|GetInstanceTransform _array_element 0 false))
              (Components|InstancedStaticMesh|UpdateInstanceTransform _array_element (- _index (LocalVariables|GetDestructionCounter)) (Math|Transform|MakeTransform (+ (.location (.OutInstanceTransform (Components|InstancedStaticMesh|GetInstanceTransform _array_element 0 false))) (Math|Vector|RotateVector (Math|Vector|MakeVector (* Delta%20Seconds (Variables|Default|GetSpeed)) 0.0 0.0) (.rotation (.OutInstanceTransform (Components|InstancedStaticMesh|GetInstanceTransform _array_element 0 false))))) (.rotation (.OutInstanceTransform (Components|InstancedStaticMesh|GetInstanceTransform _array_element 0 false))) (.scale (.OutInstanceTransform (Components|InstancedStaticMesh|GetInstanceTransform _array_element 0 false)))) false (== (- _index (LocalVariables|GetDestructionCounter)) (LocalVariables|GetLastInstanceIndex)) false)))
          (:then_1
            ;[1 1 1] Remove out-of-bounds vehicles
            (bind _returnvalue (CallFunction|IsOutOfBounds (+ (.location (.OutInstanceTransform (Components|InstancedStaticMesh|GetInstanceTransform _array_element 0 false))) (Math|Vector|RotateVector (Math|Vector|MakeVector (* Delta%20Seconds (Variables|Default|GetSpeed)) 0.0 0.0) (.rotation (.OutInstanceTransform (Components|InstancedStaticMesh|GetInstanceTransform _array_element 0 false)))))))
            (if _returnvalue
              (bind _returnvalue_2 (Class|InstancedStaticMeshComponent|RemoveInstance _array_element _index))
              (if _returnvalue_2
                (Utilities|FlowControl|Sequence
                  (:then_0
                    (Math|Integer|IncrementInt (LocalVariables|GetDestructionCounter)
                      (:%20%20
                        (bind _result (Math|Integer|DecrementInt (LocalVariables|GetLastInstanceIndex))))))
                  (:then_1
                    ;[1 1 1] Trigger update of dirty ISM since the instance we would have used was just destroyed
                    (if (== _index _result)
                      (if (> (Components|InstancedStaticMesh|GetInstanceCount _array_element) 0)
                        (Components|InstancedStaticMesh|UpdateInstanceTransform _array_element 0 (.OutInstanceTransform (Components|InstancedStaticMesh|GetInstanceTransform _array_element 0 false)) false true false)))))
                (else
                  (Development|PrintString "failed to remove instance"))))))))))

(fn Spawn
  (params (elapsed :type Float%20%28single-precision%29))
  (bind _vehicle_isms (Variables|Default|GetVehicle_ISMs))
  (bind _vehicle_isms_2 (Variables|Default|GetVehicle_ISMs))
  (bind _returnvalue (Utilities|Array|Length _vehicle_isms_2))
  (bind _returnvalue_2 (- _returnvalue 1))
  (bind _returnvalue_3 (Math|Random|RandomIntegerinRange 0 _returnvalue_2))
  (bind _output (Utilities|Array|Get(acopy) _vehicle_isms _returnvalue_3))
  (bind _returnvalue_4 (Components|InstancedStaticMesh|GetInstanceCount _output))
  (bind _returnvalue_5 (- _returnvalue_4 1))
  (for _index (range 0 _returnvalue_5)
    (for _index_2 (range 0 _returnvalue_5)
      (if (!= _index _index_2)
        (if (< (.x (.location (.OutInstanceTransform (Components|InstancedStaticMesh|GetInstanceTransform _output _index_2 false)))) (LocalVariables|GetMinDist))
          (LocalVariables|SetMinDist (LocalVariables|GetMinDist)))))
    (if (< (LocalVariables|GetMinDist) 1.4e+02)
      (Development|PrintString (Utilities|String|Append (Utilities|String|Append (Utilities|String|Append (Utilities|String|Append (Utilities|String|ToString(Float) (LocalVariables|GetMinDist)) " - elapsed: ") (Utilities|String|ToString(Float) elapsed)) "on instance ") (Utilities|String|ToString(Integer) _index_2)))))
  (Components|InstancedStaticMesh|AddInstance _output (Math|Transform|MakeTransform "0, 0, 0")))

(fn IsOutOfBounds
  (params (Location :type Vector))
  (return (> (Math|Float|Absolute(Float) (.x Location)) (Variables|Default|GetTravelDistance))))