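; BP_Log is a moving log obstacle in a top-down, lane-based game that exposes a landing point and its velocity.
; On BeginPlay it derives map and playable-zone bounds from GM_TopDown's tile layout.
; Each tick it moves forward with sweep, using a separate speed outside the playable zone, and destroys itself outside the map's Y bounds.
; Reported landing velocity is computed from forward vector and Speed, not physics.
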(event EventBeginPlay
  (Utilities|FlowControl|Sequence
    (:then_0
      (bind _asgm_top_down (Utilities|Casting|CastToGM_TopDown (Game|GetGameMode)))
      (bind _output_get (Variables|Default|SetGameMode _asgm_top_down)))
    (:then_1
      (bind _output_get_2 (Variables|Default|SetLeftMapBound (.y (Transformation|GetActorLocation (Variables|/Game/Blueprints/GM_TopDown.GM_TopDown_C|GetMapRoot _output_get)))))
      (Variables|Default|SetRightMapBound (+ _output_get_2 (* (Variables|/Game/Blueprints/GM_TopDown.GM_TopDown_C|GetMaxTilesInLane _output_get) (.y (Variables|/Game/Blueprints/GM_TopDown.GM_TopDown_C|GetTileSize _output_get)))))
      (Variables|Default|SetRightPlayableZone (+ (* (/ (Math|Conversions|ToFloat(Integer) (Variables|/Game/Blueprints/GM_TopDown.GM_TopDown_C|GetPlayableTilesInLane _output_get)) 2.0) (.y (Variables|/Game/Blueprints/GM_TopDown.GM_TopDown_C|GetTileSize _output_get))) (.y (Variables|/Game/Blueprints/GM_TopDown.GM_TopDown_C|GetTileSize _output_get))))
      (Variables|Default|SetLeftPlayableZone (* (+ (* (/ (Math|Conversions|ToFloat(Integer) (Variables|/Game/Blueprints/GM_TopDown.GM_TopDown_C|GetPlayableTilesInLane _output_get)) 2.0) (.y (Variables|/Game/Blueprints/GM_TopDown.GM_TopDown_C|GetTileSize _output_get))) (.y (Variables|/Game/Blueprints/GM_TopDown.GM_TopDown_C|GetTileSize _output_get))) -1.0)))))

(event EventTick
  (params (DeltaSeconds :type Float%20%28single-precision%29))
  (Utilities|FlowControl|Sequence
    (:then_0
      (bind _isinplayablezone (CallFunction|IsinPlayableZone))
      (if _isinplayablezone
        (Transformation|AddActorLocalOffset (Math|Vector|MakeVector (* DeltaSeconds (Variables|Default|GetSpeed)) 0.0 0.0) true false)
        (else
          (Transformation|AddActorLocalOffset (Math|Vector|MakeVector (* DeltaSeconds (Variables|Default|GetNonplayableSpeed)) 0.0 0.0) true false))))
    (:then_1
      (bind _outofbounds (CallFunction|IsOutOfBounds))
      (if _outofbounds
        (Actor|DestroyActor)))))

(fn ConstructionScript)

(fn IsinPlayableZone
  (return (Math|Float|InRange(Float) (.y (Transformation|GetActorLocation)) (Variables|Default|GetLeftPlayableZone) (Variables|Default|GetRightPlayableZone))))

(fn IsOutOfBounds
  (return (not (Math|Float|InRange(Float) (.y (Transformation|GetActorLocation)) (Variables|Default|GetLeftMapBound) (Variables|Default|GetRightMapBound)))))

(fn GetLandingPoints
  (return (Utilities|Array|MakeArray (Variables|Default|GetLandingPoint))))

(fn GetLandingPointVelocity
  (return (* (Transformation|GetActorForwardVector self) (Variables|Default|GetSpeed))))