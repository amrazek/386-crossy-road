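; BP_Train is a moving train obstacle that kills the chicken (BP_Chicken) on contact.
; Each tick it moves along its local X axis at Speed with a swept offset.
; Overlaps on any of its four train meshes feed one shared Kill call on the chicken.
; Separate swoosh and horn zones play attached pass-by sounds, without and with horn respectively, when the chicken enters them.
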(event OnComponentBeginOverlap(SM_Train1)
  (params (OverlappedComponent :type Primitive%20Component%20Object%20Reference) (OtherActor :type Actor%20Object%20Reference) (OtherComp :type Primitive%20Component%20Object%20Reference) (OtherBodyIndex :type Integer) (bFromSweep :type Boolean) (SweepResult :type Hit%20Result%20Structure%20%28by%20ref%29))
  (bind _asbp_chicken (Utilities|Casting|CastToBP_Chicken OtherActor))
  (Variables|Default|SetChicken _asbp_chicken)
  (Default|Kill (Variables|Default|GetChicken) "NewEnumerator0"))

(event OnComponentBeginOverlap(SM_Train2)
  (params (OverlappedComponent :type Primitive%20Component%20Object%20Reference) (OtherActor :type Actor%20Object%20Reference) (OtherComp :type Primitive%20Component%20Object%20Reference) (OtherBodyIndex :type Integer) (bFromSweep :type Boolean) (SweepResult :type Hit%20Result%20Structure%20%28by%20ref%29))
  (bind _asbp_chicken (Utilities|Casting|CastToBP_Chicken OtherActor))
  (Variables|Default|SetChicken _asbp_chicken)
  (Default|Kill (Variables|Default|GetChicken) "NewEnumerator0"))

(event OnComponentBeginOverlap(SM_Train3)
  (params (OverlappedComponent :type Primitive%20Component%20Object%20Reference) (OtherActor :type Actor%20Object%20Reference) (OtherComp :type Primitive%20Component%20Object%20Reference) (OtherBodyIndex :type Integer) (bFromSweep :type Boolean) (SweepResult :type Hit%20Result%20Structure%20%28by%20ref%29))
  (bind _asbp_chicken (Utilities|Casting|CastToBP_Chicken OtherActor))
  (Variables|Default|SetChicken _asbp_chicken)
  (Default|Kill (Variables|Default|GetChicken) "NewEnumerator0"))

(event OnComponentBeginOverlap(SM_Train4)
  (params (OverlappedComponent :type Primitive%20Component%20Object%20Reference) (OtherActor :type Actor%20Object%20Reference) (OtherComp :type Primitive%20Component%20Object%20Reference) (OtherBodyIndex :type Integer) (bFromSweep :type Boolean) (SweepResult :type Hit%20Result%20Structure%20%28by%20ref%29))
  (bind _asbp_chicken (Utilities|Casting|CastToBP_Chicken OtherActor))
  (Variables|Default|SetChicken _asbp_chicken)
  (Default|Kill (Variables|Default|GetChicken) "NewEnumerator0"))

(event OnComponentBeginOverlap(SwooshZone)
  (params (OverlappedComponent :type Primitive%20Component%20Object%20Reference) (OtherActor :type Actor%20Object%20Reference) (OtherComp :type Primitive%20Component%20Object%20Reference) (OtherBodyIndex :type Integer) (bFromSweep :type Boolean) (SweepResult :type Hit%20Result%20Structure%20%28by%20ref%29))
  (Utilities|Casting|CastToBP_Chicken OtherActor)
  (Audio|SpawnSoundAttached "/Game/Sounds/Train/train_pass_no_horn.train_pass_no_horn" (Variables|Default|GetDefaultSceneRoot) "None" "0, 0, 0" "0, 0, 0" "KeepRelativeOffset" false 1.0 1.0 0.0 0 0))

(event OnComponentBeginOverlap(HornZone)
  (params (OverlappedComponent :type Primitive%20Component%20Object%20Reference) (OtherActor :type Actor%20Object%20Reference) (OtherComp :type Primitive%20Component%20Object%20Reference) (OtherBodyIndex :type Integer) (bFromSweep :type Boolean) (SweepResult :type Hit%20Result%20Structure%20%28by%20ref%29))
  (Utilities|Casting|CastToBP_Chicken OtherActor)
  (Audio|SpawnSoundAttached "/Game/Sounds/Train/train_pass_shorter.train_pass_shorter" (Variables|Default|GetDefaultSceneRoot) "None" "0, 0, 0" "0, 0, 0" "KeepRelativeOffset" false 1.0 1.0 0.0 0 0))

(event EventTick
  (params (DeltaSeconds :type Float%20%28single-precision%29))
  (Transformation|AddActorLocalOffset (Math|Vector|MakeVector (* DeltaSeconds (Variables|Default|GetSpeed)) 0.0 0.0) true false))

(fn ConstructionScript)