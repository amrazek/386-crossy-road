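; BP_LogSpawner repeatedly spawns moving BP_Log actors at its map-aligned location, using the spawner's rotation and scale.
; A non-looping timer re-arms itself on each spawn with a random delay between MinDelay and MaxDelay.
; Logs receive separate playable and unplayable speeds and are not spawned when colliding.
; The random variant switch is vestigial: its range is fixed at 1, and every case spawns the same log.
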(event Custom|SpawnLog
  (bind _returnvalue (Transformation|GetActorTransform))
  (Utilities|Time|ClearandInvalidateTimerbyHandle (stale _returnvalue_2))
  (Utilities|FlowControl|Sequence
    (:then_0
      (bind _returnvalue_2 (Utilities|Time|SetTimerbyEvent (delegate Custom|SpawnLog) (Math|Random|RandomFloatinRange (Variables|Default|GetMinDelay) (Variables|Default|GetMaxDelay)))))
    (:then_1
      (bind _alignedworldposition (CallFunction|GetMapAlignedPosition (.location _returnvalue) (Variables|Default|GetGameMode))))
    (:then_2
      (switch int (Math|Random|RandomIntegerinRange 1 1)
        (:1
          _)
        (:2
          _)
        (:3
          _))
      (Game|SpawnActorfromClass "/Game/Blueprints/ObstacleSpawners/BP_Log.BP_Log_C" (Math|Transform|MakeTransform _alignedworldposition (.rotation _returnvalue) (.scale _returnvalue)) "DontSpawnIfColliding" 0 (Variables|Default|GetLogPlayableSpeed) (Variables|Default|GetLogUnplayableSpeed) 0))))

(event EventBeginPlay
  (Utilities|FlowControl|Sequence
    (:then_0
      (bind _asgm_top_down (Utilities|Casting|CastToGM_TopDown (Game|GetGameMode)))
      (Variables|Default|SetGameMode _asgm_top_down))
    (:then_1
      (bind _returnvalue (Utilities|Time|SetTimerbyEvent (delegate Custom|SpawnLog) (Math|Random|RandomFloatinRange (Variables|Default|GetMinDelay) (Variables|Default|GetMaxDelay)))))))

(fn ConstructionScript)

(fn Seed)