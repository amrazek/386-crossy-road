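; BP_TrainSpawner is an obstacle spawner that repeatedly spawns BP_Train actors at its own transform, starting on BeginPlay.
; Each spawn passes in TrainSpeed, skips if colliding, and re-arms a one-shot timer with a random delay between MinTime and MaxTime.
; Train lifespan is lane length from GM_TopDown's tile size and tile count, plus a fixed margin, divided by speed.
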(event Custom|SpawnTrain
  (bind _gamemode (Variables|Default|GetGameMode))
  (bind _returnvalue (Game|SpawnActorfromClass "/Game/Blueprints/ObstacleSpawners/BP_Train.BP_Train_C" (Transformation|GetActorTransform) "DontSpawnIfColliding" 0 (Variables|Default|GetTrainSpeed) 0))
  (Actor|SetLifeSpan _returnvalue (/ (+ (* (.y (Variables|/Game/Blueprints/GM_TopDown.GM_TopDown_C|GetTileSize _gamemode)) (Math|Conversions|ToFloat(Integer) (Variables|/Game/Blueprints/GM_TopDown.GM_TopDown_C|GetMaxTilesInLane _gamemode))) 1.5e+03) (Variables|Default|GetTrainSpeed)))
  (Utilities|Time|SetTimerbyEvent (delegate Custom|SpawnTrain) (Math|Random|RandomFloatinRange (Variables|Default|GetMinTime) (Variables|Default|GetMaxTime))))

(event EventBeginPlay
  (Utilities|FlowControl|Sequence
    (:then_0
      (bind _asgm_top_down (Utilities|Casting|CastToGM_TopDown (Game|GetGameMode)))
      (Variables|Default|SetGameMode _asgm_top_down))
    (:then_1
      (Utilities|Time|SetTimerbyEvent (delegate Custom|SpawnTrain) (Math|Random|RandomFloatinRange (Variables|Default|GetMinTime) (Variables|Default|GetMaxTime)) :!label _label))
    (:then_2
      (bind _returnvalue (Game|SpawnActorfromClass "/Game/Blueprints/ObstacleSpawners/BP_Train.BP_Train_C" (Transformation|GetActorTransform) "DontSpawnIfColliding" 0 (Variables|Default|GetTrainSpeed) 0))
      (Actor|SetLifeSpan _returnvalue (/ (+ (* (.y (Variables|/Game/Blueprints/GM_TopDown.GM_TopDown_C|GetTileSize (Variables|Default|GetGameMode))) (Math|Conversions|ToFloat(Integer) (Variables|/Game/Blueprints/GM_TopDown.GM_TopDown_C|GetMaxTilesInLane (Variables|Default|GetGameMode)))) 1.5e+03) (Variables|Default|GetTrainSpeed)))
      (goto _label))))

(fn ConstructionScript)